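; Mission boundary volume that damages the player who stays outside it too long.
; Leaving sets OutsideMissionArea on the overlapping Bp_Marine and starts a timer lasting SecondsBeforePlayerDeath, while re-entering clears both.
; When the timer expires, Kill Player applies fixed damage to player character 0, regardless of which marine left.
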(event EventBeginPlay)

(event Collision|EventActorBeginOverlap
  (params (OtherActor :type Actor%20Object%20Reference))
  (bind _asbp_marine (Utilities|Casting|CastToBp_Marine OtherActor))
  (Variables|/Game/Blueprints/Pawns/Bp_Marine.Bp_Marine_C|SetOutside%20Mission%20Area _asbp_marine false)
  (Utilities|Time|ClearTimerbyFunctionName 0 "Kill Player"))

(event EventTick
  (params (DeltaSeconds :type Float%20%28single-precision%29)))

(event Collision|EventActorEndOverlap
  (params (OtherActor :type Actor%20Object%20Reference))
  (bind _asbp_marine (Utilities|Casting|CastToBp_Marine OtherActor))
  (Variables|/Game/Blueprints/Pawns/Bp_Marine.Bp_Marine_C|SetOutside%20Mission%20Area _asbp_marine true)
  (Utilities|Time|SetTimerbyFunctionName 0 "Kill Player" (Variables|Default|Getseconds%20before%20player%20death)))

(fn ConstructionScript)

(fn KillPlayer
  (Game|Damage|ApplyDamage (Game|GetPlayerCharacter 0) 1e+02 0 0))