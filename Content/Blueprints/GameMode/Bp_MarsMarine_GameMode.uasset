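; Game mode for Mars Marine that runs endless, escalating waves of alien enemies.
; Each wave multiplies the alien count by a difficulty multiplier and shortens the clamped spawn interval, driving a looping named timer.
; The timer spawns aliens at random TargetPoints until the quota runs out.
; Registered deaths remove aliens from the tracked list, and an empty list with no spawns remaining starts the next wave after a short delay.
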(event Custom|End%20Wave
  (Utilities|FlowControl|Delay 2.0)
  (CallFunction|StartNewWave))

(event Custom|Spawn%20Wave
  (CallFunction|SpawnAlien))

(event EventTick
  (params (DeltaSeconds :type Float%20%28single-precision%29)))

(event EventBeginPlay
  (Utilities|FlowControl|Delay 2.0)
  (CallFunction|StartNewWave))

(fn ConstructionScript)

(fn StartNewWave
  (Math|Integer|IncrementInt (Variables|Default|GetCurrent%20Wave)
    (:%20%20
      (bind _returnvalue (CallFunction|IncreaseWaveDifficulty))
      (Utilities|Time|SetTimerbyFunctionName 0 "Spawn Wave" _returnvalue true))))

(fn SpawnAlien
  (bind _random_spawn_point (CallFunction|GetRandomSpawnPoint))
  (Utilities|IsValid _random_spawn_point
    (:Is%20Valid
      (bind _returnvalue (Game|SpawnActorfromClass "/Game/Blueprints/Ai/Bp_Alien.Bp_Alien_C" (Transformation|GetActorTransform _random_spawn_point) "Undefined" 0 0))
      (Utilities|IsValid _returnvalue
        (:Is%20Valid
          (Utilities|Array|Add (Variables|Default|GetAliens) _returnvalue)
          (bind _result (Math|Integer|DecrementInt (Variables|Default|GetAliens%20Spawns%20Remaing))
            (:%20%20
              (if (== _result 0)
                (Utilities|Time|ClearTimerbyFunctionName 0 "Spawn Wave")))))))))

(fn GetRandomSpawnPoint
  (bind _outactors (Actor|GetAllActorsOfClass "/Script/Engine.TargetPoint"))
  (return (Utilities|Array|Get(acopy) _outactors (Math|Random|RandomIntegerinRange 0 (Utilities|Array|LastIndex _outactors)))))

(fn RegisterAlienDeath
  (params (Alien :type Bp%20Alien%20Object%20Reference%20%28by%20ref%29))
  (Utilities|Array|RemoveItem (Variables|Default|GetAliens) Alien)
  (if (CallFunction|IsWaveComplete)
    (CallFunction|EndWave)))

(fn IsWaveComplete
  (return (and (== (Utilities|Array|Length (Variables|Default|GetAliens)) 0) (== (Variables|Default|GetAliens%20Spawns%20Remaing) 0))))

(fn IncreaseWaveDifficulty
  (bind _output_get (Variables|Default|SetWave%20Difficulty (Math|Float|Round (* (Variables|Default|GetWave%20Difficulty) (Variables|Default|GetDifficulty%20Multiplier)))))
  (Variables|Default|SetAliens%20Spawns%20Remaing _output_get)
  (bind _returnvalue (CallFunction|DecreaseAlienSpawnTime))
  (return _returnvalue))

(fn DecreaseAlienSpawnTime
  (bind _output_get (Variables|Default|SetSpawn%20Times (Math|Float|Clamp(Float) (/ (Variables|Default|GetSpawn%20Times) 1.05) 0.25)))
  (return _output_get))