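; Alien enemy AI character that chases the player's marine and makes melee attacks.
; A repeating AIMoveTo loop drives pursuit, while Tick checks range and state, then halts movement during the attack montage.
; DamagePlayer applies hit damage but is not called within this Blueprint.
; Incoming damage lowers clamped health; at zero the alien disables collision, credits the marine's kill, notifies the game mode and is destroyed after a delay.
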(event EventBeginPlay
  (if (CallFunction|IsAiAlive) :!label _label
    (AI|AIMoveTo self "0, 0, 0" (Game|GetPlayerCharacter 0) 5.0 false
      (:OnSuccess
        _)
      (:OnFail
        _))
    (Utilities|FlowControl|Delay 0.2)
    (goto _label)))

(event Collision|EventActorBeginOverlap
  (params (OtherActor :type Actor%20Object%20Reference)))

(event EventTick
  (params (DeltaSeconds :type Float%20%28single-precision%29))
  (if (CallFunction|CanAttack)
    (CallFunction|DeactivateAiMovement)
    (Animation|Montage|PlayMontage (Variables|Character|GetMesh) "/Game/Characters/Enemy_Great_Spider/Animations/AlieanAttack1.AlieanAttack1"
      (:OnCompleted
        (CallFunction|ActivateAiMovement)))))

(event Game|Damage|EventAnyDamage
  (params (Damage :type Float%20%28single-precision%29) (DamageType :type Damage%20Type%20Object%20Reference) (InstigatedBy :type Controller%20Object%20Reference) (DamageCauser :type Actor%20Object%20Reference))
  (if (CallFunction|IsAiAlive)
    (bind _health (CallFunction|DecreaseHealthbyAmountOfDamage Damage))
    (if (== _health 0.0)
      (CallFunction|KillAi)
      (Utilities|FlowControl|Delay 3.0)
      (Actor|DestroyActor))))

(fn ConstructionScript)

(fn IsWithinAttackRange
  (return (< (Transformation|GetDistanceTo (Game|GetPlayerCharacter 0)) (Variables|Default|GetAttack%20Range))))

(fn IsAttacking
  (return (Animation|Montage|MontageIsPlaying (Components|SkeletalMesh|GetAnimInstance (Variables|Character|GetMesh)) "/Game/Characters/Enemy_Great_Spider/Animations/AlieanAttack1.AlieanAttack1")))

(fn DeactivateAiMovement
  (bind _charactermovement (Variables|Character|GetCharacterMovement))
  (Components|Movement|StopMovementImmediately _charactermovement)
  (Components|Activation|Deactivate _charactermovement))

(fn ActivateAiMovement
  (Components|Activation|Activate (Variables|Character|GetCharacterMovement) false))

(fn DamagePlayer
  (if (CallFunction|IsAiAlive)
    (Game|Damage|ApplyDamage (Game|GetPlayerCharacter 0) (Variables|Default|GetDamage%20Per%20Hit) 0 0)))

(fn DecreaseHealthbyAmountOfDamage
  (params (Damage%20Alien :type Float%20%28single-precision%29))
  (bind _output_get (Variables|Default|SetHealth (Math|Float|Clamp(Float) (- (Variables|Default|GetHealth) Damage%20Alien) 0.0 1e+02)))
  (return _output_get))

(fn KillAi
  (Variables|Default|SetDead true)
  (CallFunction|DeactivateAiMovement)
  (Collision|SetActorEnableCollision false)
  (bind _asbp_marine (Utilities|Casting|CastToBp_Marine (Game|GetPlayerCharacter 0)))
  (Default|IncreaseKills _asbp_marine)
  (bind _asbp_mars_marine_game_mode (Utilities|Casting|CastToBp_MarsMarine_GameMode (Game|GetGameMode)))
  (Default|RegisterAlienDeath _asbp_mars_marine_game_mode self))

(fn IsAiAlive
  (return (not (Variables|Default|GetDead))))

(fn CanAttack
  (bind _asbp_marine (Utilities|Casting|CastToBp_Marine (Game|GetPlayerCharacter 0)))
  (return (Math|Boolean|ANDBoolean (CallFunction|IsAiAlive) (CallFunction|IsWithinAttackRange) (not (CallFunction|IsAttacking)) (Default|IsPlayerAlive _asbp_marine))))